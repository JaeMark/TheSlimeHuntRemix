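; Base projectile actor that flies with muzzle, projectile and hit-impact particle effects and damages overlapped actors carrying a target tag.
; Construction applies speed, collider radius, rotation, scale and optional color to the components and effects.
; BeginPlay fires the muzzle effect and, given a warm-up time, hides and halts the projectile until it elapses.
; A tagged hit plays the impact, stops the projectile immediately or after its lifespan, then destroys the actor.
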(event Custom|SpawnMuzzle
  (bind _muzzle (Variables|Default|GetMuzzle))
  (Effects|Components|ParticleSystem|SetTemplate _muzzle (Variables|Components|GetVFXMuzzle))
  (Transformation|SetWorldLocation _muzzle (+ (Transformation|GetActorLocation) (Variables|Components|GetMuzzleOffset)) false false))

(event Custom|SpawnProjectile
  (Effects|Components|ParticleSystem|SetTemplate (Variables|Default|GetProjectile) (Variables|Components|GetVFXProjectile))
  (Game|Components|ProjectileMovement|SetVelocityinLocalSpace (Variables|Default|GetProjectileMovement) (Variables|Components|GetoriginalVelocity)))

(event Custom|StopProjectile
  (Components|Activation|Deactivate (Variables|Default|GetProjectile))
  (Components|Movement|StopMovementImmediately (Variables|Default|GetProjectileMovement)))

(event Custom|SetProjectileTemplateToEmpty
  (Effects|Components|ParticleSystem|SetTemplate (Variables|Default|GetProjectile) 0)
  (Components|Movement|StopMovementImmediately (Variables|Default|GetProjectileMovement)))

(event EventBeginPlay
  (bind _warmuptime (Variables|Components|GetWarmUpTime))
  (Variables|Components|SetoriginalVelocity (Variables|/Script/Engine.MovementComponent|GetVelocity (Variables|Default|GetProjectileMovement)))
  (Variables|Components|SetoriginalLocation (Transformation|GetWorldLocation (Variables|Default|GetDefaultSceneRoot)))
  (CallFunction|SpawnMuzzle)
  (if (> _warmuptime 0.0)
    (CallFunction|SetProjectileTemplatetoEmpty)
    (Utilities|FlowControl|Delay _warmuptime)
    (CallFunction|SpawnProjectile)))

(event Collision|EventActorBeginOverlap
  (params (OtherActor :type Actor%20Object%20Reference))
  (bind _hit (Variables|Default|GetHit))
  (Variables|Default|SetTarget OtherActor)
  (if (Actor|ActorHasTag OtherActor (Variables|Default|GetTargetTag))
    (Game|Damage|ApplyDamage (Variables|Default|GetTarget) (Variables|Components|GetDeltaHealth) 0 self)
    (Effects|Components|ParticleSystem|SetTemplate _hit (Variables|Components|GetVFXHit/Impact))
    (Transformation|SetWorldLocation _hit (+ (Math|Transform|TransformLocation (Transformation|GetActorTransform) "0, 0, 0") (Variables|Components|GetHit/ImpactOffset)) false false)
    (if (Variables|Default|GetIsDestroyedOnImpact)
      _
      (else
        (Utilities|FlowControl|Delay (Variables|Components|GetProjectileLifeSpan))))
    (CallFunction|StopProjectile)
    (Components|DestroyComponent (Variables|Default|GetProjectileCollider))
    (Utilities|FlowControl|Delay 2.0)
    (Actor|DestroyActor)))

(fn ConstructionScript
  (bind _scale (Variables|Components|GetScale))
  (bind _scale_2 (Variables|Components|GetScale))
  (bind _projectile (Variables|Default|GetProjectile))
  (bind _scale_3 (Variables|Components|GetScale))
  (bind _hit (Variables|Default|GetHit))
  (bind _muzzle (Variables|Default|GetMuzzle))
  (bind _color (Variables|Components|GetColor))
  (Variables|/Script/Engine.ProjectileMovementComponent|SetInitialSpeed (Variables|Default|GetProjectileMovement) (Variables|Components|GetProjectileSpeed))
  (Components|Sphere|SetSphereRadius (Variables|Default|GetProjectileCollider) (Variables|Components|GetColliderRadius) true)
  (Effects|Components|ParticleSystem|SetTemplate (Variables|Default|GetProjectile) (Variables|Components|GetVFXProjectile))
  (Variables|/Script/Engine.RotatingMovementComponent|SetRotationRate (Variables|Default|GetRotatingMovement) (Variables|Components|GetRotationRate))
  (if (Variables|Components|GetbChangeColor)
    (Effects|Components|ParticleSystem|SetColorParameter (Variables|Default|GetProjectile) "Color" _color)
    (Effects|Components|ParticleSystem|SetColorParameter (Variables|Default|GetHit) "Color" _color)
    (Effects|Components|ParticleSystem|SetColorParameter (Variables|Default|GetMuzzle) "Color" _color))
  (Effects|Components|ParticleSystem|SetVectorParameter _projectile "Scale" _scale_2)
  (Effects|Components|ParticleSystem|SetFloatParameter _projectile "Scale" (.X (Math|Vector|BreakVector _scale_2)))
  (Effects|Components|ParticleSystem|SetVectorParameter _hit "Scale" _scale_3)
  (Effects|Components|ParticleSystem|SetFloatParameter _hit "Scale" (.X (Math|Vector|BreakVector _scale_3)))
  (Effects|Components|ParticleSystem|SetVectorParameter _muzzle "Scale" _scale)
  (Effects|Components|ParticleSystem|SetFloatParameter _muzzle "Scale" (.X (Math|Vector|BreakVector _scale))))