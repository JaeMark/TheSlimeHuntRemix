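; BP_CheckPointPlant is a plant checkpoint that registers itself with BP_GameMode and respawns the player from the plant.
; Overlap by the player character plays a sound, sets it as the current checkpoint, then after a short delay swaps the plant's material and disables checkpoint collision.
; RespawnPlayer destroys the old character, spawns and possesses a new one at the plant, then launches it along SpawnPoint's forward vector after a delay.
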(event EventBeginPlay
  (bind _asbp_game_mode (Utilities|Casting|CastToBP_GameMode (Game|GetGameMode)))
  (Variables|Default|SetGameMode _asbp_game_mode))

(event Collision|EventActorBeginOverlap
  (params (OtherActor :type Actor%20Object%20Reference))
  (if (== OtherActor "/Game/Blueprints/BP_PlayerCharacter.BP_PlayerCharacter")
    (Audio|PlaySound2D "/Game/Audio/harp-set-3-97810.harp-set-3-97810" 1.0 1.0 0.0 0 0)
    (Variables|/Game/Blueprints/BP_GameMode.BP_GameMode_C|SetCurrentCheckpoint (Variables|Default|GetGameMode) self)
    (Utilities|FlowControl|Delay 0.2)
    (Rendering|Material|SetMaterial (Variables|Default|GetPlant) 0 "/Paper2D/TranslucentUnlitSpriteMaterial.TranslucentUnlitSpriteMaterial")
    (Collision|SetCollisionEnabled (Variables|Default|GetCheckpoint) "NoCollision")))

(event EventRespawnPlayer
  (params (Player :type Actor%20Object%20Reference))
  (Utilities|IsValid Player
    (:Is%20Valid
      (Actor|DestroyActor Player))
    (:Is%20Not%20Valid
      _))
  (bind _returnvalue (Game|SpawnActorfromClass "/Game/Blueprints/BP_PlayerCharacter.BP_PlayerCharacter_C" (Math|Transform|MakeTransform (Transformation|GetWorldLocation (Variables|Default|GetPlant)) "0, 0, 0" "1.000000,1.000000,1.000000") "Undefined" "MultiplyWithRoot" 0 0))
  (bind _output_get (Variables|Default|SetPlayer _returnvalue))
  (Pawn|Possess (Game|GetPlayerController 0) _output_get)
  (Utilities|FlowControl|Delay 1.0)
  (Class|BPILaunchActor|LaunchActor(Message) (Variables|Default|GetPlayer) (Math|Vector|GetForwardVector (Variables|Default|GetSpawnPoint)) (Variables|Default|GetLaunchVelocityMagitude)))

(fn ConstructionScript)