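; BP_EndGoal is the goal actor that ends the game when the player reaches it.
; On BeginPlay it caches the BP_PlayerCharacter for player 0.
; When that character overlaps it, it pauses the game and adds a WBP_EndScreen widget to the viewport.
; A "Remove HUD" branch is present but disconnected, so it never runs.
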(event Collision|EventActorBeginOverlap
  (params (OtherActor :type Actor%20Object%20Reference))
  (if (== OtherActor (Variables|Default|GetPlayer))
    ;[1 1 1] Display End Screen
    (Game|SetGamePaused true)
    (bind _returnvalue (UserInterface|CreateWidget "/Game/HUD/WBP_EndScreen.WBP_EndScreen_C"))
    (UserInterface|Viewport|AddtoViewport _returnvalue 0)))

(event EventBeginPlay
  (bind _asbp_player_character (Utilities|Casting|CastToBP_PlayerCharacter (Game|GetPlayerCharacter 0)))
  (Variables|Default|SetPlayer _asbp_player_character))

(fn ConstructionScript)