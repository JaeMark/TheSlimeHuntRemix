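; BP_Slime is a collectible slime pickup actor that the player gathers by touching it.
; It plays a quiet spawn sound at its location on BeginPlay.
; On overlap with BP_PlayerCharacter, it plays one of two random cheer sounds, waits briefly, increments the slime count on BP_GameMode, then destroys itself.
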(event EventBeginPlay
  (Audio|PlaySoundatLocation "/Game/Audio/slime-71707.slime-71707" (Transformation|GetActorLocation) "0, 0, 0" 0.2 1.0 0.0 0 0 0 0))

(event Collision|EventActorBeginOverlap
  (params (OtherActor :type Actor%20Object%20Reference))
  (Utilities|Casting|CastToBP_PlayerCharacter OtherActor)
  (Audio|PlaySound2D (Utilities|Select :Index (Math|Random|RandomIntegerinRange 0 1) :Option%200 "/Game/Audio/yipee-45360.yipee-45360" :Option%201 "/Game/Audio/yay-6120.yay-6120") 0.5 1.0 0.0 0 0)
  (Utilities|FlowControl|Delay 0.2)
  (bind _asbp_game_mode (Utilities|Casting|CastToBP_GameMode (Game|GetGameMode)))
  (Default|IncrementSlimeCount _asbp_game_mode)
  (Actor|DestroyActor))

(fn ConstructionScript)