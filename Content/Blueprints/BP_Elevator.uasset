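; BP_Elevator is an elevator actor with a tile map Platform that starts a scripted sequence when the player character steps into it.
; BeginPlay assigns the elevator tile map to the Platform.
; The first player overlap sets IsMoving, starts a camera shake, and after a short delay creates and plays the elevator Level Sequence.
; IsMoving is never reset here, so the trigger fires only once.
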(event EventBeginPlay
  (Class|PaperTileMapComponent|SetTileMap (Variables|Default|GetPlatform) "/Game/Tilemaps/TM_Elevator.TM_Elevator"))

(event Collision|EventActorBeginOverlap
  (params (OtherActor :type Actor%20Object%20Reference))
  (if (and (== OtherActor (Game|GetPlayerCharacter 0)) (not (Variables|Default|GetbIsMoving)))
    (Variables|Default|SetbIsMoving true)
    (CameraShakes|StartCameraShake (Game|GetPlayerCameraManager 0) "/Game/Blueprints/CameraShakes/CS_Elevator.CS_Elevator_C" 1.0 "CameraLocal" "0, 0, 0")
    (Utilities|FlowControl|Delay 2.0)
    (bind _returnvalue (Sequencer|Player|CreateLevelSequencePlayer "/Game/LevelSequences/LS_Elevator.LS_Elevator"))
    (bind _output_get (Variables|Default|SetSequencePlayer _returnvalue))
    (Sequencer|Player|Play _output_get :!class /Script/MovieScene.MovieSceneSequencePlayer)))

(fn ConstructionScript)