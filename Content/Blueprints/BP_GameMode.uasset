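; Game mode that tracks the player's current plant checkpoint and collected slime count, and handles respawns and elevator resets.
; On begin play it takes the "Start"-tagged checkpoint plant as current, spawns the player there and swaps that plant's material.
; RespawnPlayer delegates to the current checkpoint, while IncrementSlimeCount bumps the slime tally.
; Reset stops every elevator's sequence player and clears its moving flag.
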(event Custom|IncrementSlimeCount
  ;[1 1 1] Increment Collected Slime Count
  (bind _result (Math|Integer|IncrementInt (Variables|Default|GetCollectedSlimes))
    (:%20%20
      (Variables|Default|SetCollectedSlimes _result))))

(event Custom|RespawnPlayer
  ;[1 1 1] Respawns Player
  (bind _asbp_check_point_plant (Utilities|Casting|CastToBP_CheckPointPlant (Variables|Default|GetCurrentCheckpoint)))
  (Default|RespawnPlayer _asbp_check_point_plant))

(event Custom|Reset
  ;[1 1 1] Resets Elevator Platform
  (bind _outactors (Actor|GetAllActorsOfClass "/Game/Blueprints/BP_Elevator.BP_Elevator_C"))
  (for _array_element _outactors
    (bind _output_get (Variables|Default|SetElevator _array_element))
    (Utilities|IsValid (Variables|/Game/Blueprints/BP_Elevator.BP_Elevator_C|GetSequencePlayer _output_get)
      (:Is%20Valid
        (Sequencer|Player|Stop (Variables|/Game/Blueprints/BP_Elevator.BP_Elevator_C|GetSequencePlayer _output_get) :!class /Script/MovieScene.MovieSceneSequencePlayer)
        (Variables|/Game/Blueprints/BP_Elevator.BP_Elevator_C|SetbIsMoving (Variables|Default|GetElevator) false)))))

(event EventBeginPlay
  ;[1 1 1] Set Plant Spawn Point
  (bind _outactors (Actor|GetAllActorsOfClasswithTag "/Game/Blueprints/BP_CheckPointPlant.BP_CheckPointPlant_C" "Start"))
  (Variables|Default|SetCurrentCheckpoint (Utilities|Array|Get(acopy) _outactors))
  (Default|RespawnPlayer (Utilities|Array|Get(acopy) _outactors))
  (Rendering|Material|SetMaterial (Variables|/Game/Blueprints/BP_CheckPointPlant.BP_CheckPointPlant_C|GetPlant (Utilities|Array|Get(acopy) _outactors)) 0 "/Paper2D/TranslucentUnlitSpriteMaterial.TranslucentUnlitSpriteMaterial"))

(fn ConstructionScript)