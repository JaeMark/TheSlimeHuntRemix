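; BP_ChallengeGameMode is a game mode that handles checkpoint respawning and background music for a challenge level.
; On BeginPlay it starts the music, stores the plant checkpoint tagged "Start" as current, spawns the player there and changes that plant's material.
; HandlePlayerDeath sends a respawn message to the current checkpoint.
; PlayEndMusic stops the background track and plays the ending track.
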(event Custom|PlayEndMusic
  (Audio|Components|Audio|Stop (Variables|Default|GetBGMusic))
  (Audio|PlaySound2D "/Game/FantasyOrchestral/audio/Elven_Realm.Elven_Realm" 1.0 1.0 0.0 0 0))

(event EventBeginPlay
  (Utilities|FlowControl|Sequence
    (:then_0
      (bind _returnvalue (Audio|SpawnSound2D "/Game/FantasyOrchestral/cues/LandOfMystery.LandOfMystery" 0.5 1.0 0.0 0))
      (Variables|Default|SetBGMusic _returnvalue))
    (:then_1
      ;[1 1 1] Set Plant Spawn Point
      (bind _outactors (Actor|GetAllActorsOfClasswithTag "/Game/Blueprints/BP_CheckPointPlant.BP_CheckPointPlant_C" "Start"))
      (Variables|Default|SetCurrentCheckpoint (Utilities|Array|Get(acopy) _outactors))
      (Class|BPIRespawnPlayer|RespawnPlayer(Message) (Variables|Default|GetCurrentCheckpoint) (Game|GetPlayerCharacter 0))
      (Rendering|Material|SetMaterial (Variables|/Game/Blueprints/BP_CheckPointPlant.BP_CheckPointPlant_C|GetPlant (Utilities|Array|Get(acopy) _outactors)) 0 "/Paper2D/TranslucentUnlitSpriteMaterial.TranslucentUnlitSpriteMaterial"))))

(event EventHandlePlayerDeath
  (params (Player :type Actor%20Object%20Reference))
  ;[1 1 1] Respawns Player
  (Class|BPIRespawnPlayer|RespawnPlayer(Message) (Variables|Default|GetCurrentCheckpoint) Player))

(fn ConstructionScript)