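; BP_HostileSlime is a sprite-based enemy slime character that damages any Player-tagged actor it overlaps.
; Incoming damage lowers clamped health, updates a widget health bar, and either briefly flickers the sprite with a pitch-randomized sound or triggers death.
; Death detaches the controller, disables capsule collision, plays sound and a tinted particle burst, then hides and destroys the slime.
; A LaunchActor event lets it be knocked in a given direction.
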(event EventBeginPlay
  (Utilities|FlowControl|Sequence
    (:then_0
      (Audio|PlaySoundatLocation "/Game/Audio/slime-71707.slime-71707" (Transformation|GetActorLocation) "0, 0, 0" 0.2 1.0 0.0 0 0 0 0)
      (Variables|Default|SetHealth (Variables|Default|GetMaxHealth)))
    (:then_1
      (bind _aswbp_health (Utilities|Casting|CastToWBP_Health (UserInterface|GetWidget (Variables|Default|GetHealthWidget))))
      (Variables|Default|SetHealthWidgetRef _aswbp_health)
      (CallFunction|OnHealthUpdate))
    (:then_2
      (Variables|Default|SetOriginal%20Sprite%20Color (Variables|/Script/Paper2D.PaperFlipbookComponent|GetSpriteColor (Variables|Default|GetSlime))))))

(event Collision|EventActorBeginOverlap
  (params (OtherActor :type Actor%20Object%20Reference))
  (if (Actor|ActorHasTag OtherActor "Player")
    (Game|Damage|ApplyDamage OtherActor (Variables|Default|GetDamage) 0 0)))

(event Game|Damage|EventAnyDamage
  (params (Damage :type Float%20%28single-precision%29) (DamageType :type Damage%20Type%20Object%20Reference) (InstigatedBy :type Controller%20Object%20Reference) (DamageCauser :type Actor%20Object%20Reference))
  (bind _returnvalue (Transformation|GetActorLocation))
  ;[1 1 1] Calculate health after damage
  (bind _output_get (Variables|Default|SetHealth (Math|Float|Clamp(Float) (- (Variables|Default|GetHealth) Damage) 0.0 (Variables|Default|GetMaxHealth))))
  (CallFunction|OnHealthUpdate)
  (if (<= _output_get 0.0)
    (Class|Pawn|DetachfromControllerPendingDestroy)
    (Collision|SetCollisionProfileName (Variables|Collision|GetCapsuleComponent) "NoCollision" true :!class /Script/Engine.PrimitiveComponent)
    ;[1 1 1] Play death VFX and SFX
    (Audio|PlaySoundatLocation "/Game/GameDevelopment1/Audio/Dark_Fantasy_Studio-Crawler_18.Dark_Fantasy_Studio-Crawler_18" _returnvalue "0, 0, 0" 0.4 1.0 0.0 0 0 0 0)
    (bind _returnvalue_2 (Effects|SpawnEmitteratLocation "/Game/MagicProjectilesVol2/Particles/Hits/P_Hit_Waterball01_Blue.P_Hit_Waterball01_Blue" _returnvalue "0, 0, 0" "2.000000,2.000000,2.000000"))
    (Effects|Components|ParticleSystem|SetColorParameter _returnvalue_2 "Color" "(R=0.366253,G=0.212231,B=0.084376,A=1.000000)")
    (Rendering|SetActorHiddenInGame true)
    (Utilities|FlowControl|Delay 0.5)
    (Actor|DestroyActor)
    (else
      (Audio|PlaySoundatLocation "/Game/GameDevelopment1/Audio/slimejump-6913.slimejump-6913" (Transformation|GetActorLocation) "0, 0, 0" 0.2 (Math|Random|RandomFloatinRange 0.0 0.75) 0.0 0 0 0 0)
      ;[1 1 1] Flicker sprite when damaged
      (Sprite|SetSpriteColor (Variables|Default|GetSlime) (Variables|Default|GetFlicker%20Sprite%20Color))
      (Utilities|FlowControl|Delay 0.25)
      (Sprite|SetSpriteColor (Variables|Default|GetSlime) (Variables|Default|GetOriginal%20Sprite%20Color)))))

(event EventLaunchActor
  (params (Direction :type Vector :default "0, 0, 0") (LaunchIntensity :type Float%20%28double-precision%29))
  (Character|LaunchCharacter (* Direction LaunchIntensity) true true))

(fn ConstructionScript)

(fn OnHealthUpdate
  (Variables|/Script/UMG.ProgressBar|SetPercent (Variables|/Game/GameDevelopment1/Widgets/WBP_Health.WBP_Health_C|GetHealth (Variables|Default|GetHealthWidgetRef)) (/ (Variables|Default|GetHealth) (Variables|Default|GetMaxHealth))))