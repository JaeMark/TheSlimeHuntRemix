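; Base projectile actor with muzzle, travel and impact VFX, configured in the construction script.
; An optional warm-up holds it hidden and still, then restores its velocity and starts a lifespan timer.
; Expiry, or overlap with anything not tagged Player or Projectile (which adds camera shake), triggers the explosion.
; A sphere trace launches BPI_LaunchActor implementers away in the XZ plane before the actor is destroyed.
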(event OnComponentBeginOverlap(ProjectileCollider)
  (params (OverlappedComponent :type Primitive%20Component%20Object%20Reference) (OtherActor :type Actor%20Object%20Reference) (OtherComp :type Primitive%20Component%20Object%20Reference) (OtherBodyIndex :type Integer) (bFromSweep :type Boolean) (SweepResult :type Hit%20Result%20Structure%20%28by%20ref%29))
  ;[1 1 1] Explode on impact if projectile overlaps with an actor that is not the player or another projectile
  (if (and (not (Actor|ActorHasTag OtherActor "Player")) (not (Actor|ActorHasTag OtherActor "Projectile")))
    (Variables|Default|SetTarget OtherActor)
    (CameraShakes|StartCameraShake (Game|GetPlayerCameraManager 0) "/Game/GameDevelopment1/Blueprints/ScreenShakes/CS_ProjectileImpact.CS_ProjectileImpact_C" 1.0 "CameraLocal" "0, 0, 0")
    (Utilities|Time|ClearTimerbyFunctionName 0 "DestroyProjectile")
    (CallFunction|DestroyProjectile)))

(event Custom|SpawnMuzzle
  (bind _muzzle (Variables|Default|GetMuzzle))
  ;[1 1 1] Projectile component setup
  (Effects|Components|ParticleSystem|SetTemplate _muzzle (Variables|Components|GetVFXMuzzle))
  (Transformation|SetWorldLocation _muzzle (+ (Transformation|GetActorLocation) (Variables|Components|GetMuzzleOffset)) false false))

(event Custom|SpawnProjectile
  ;[1 1 1] Projectile component setup
  (Effects|Components|ParticleSystem|SetTemplate (Variables|Default|GetProjectile) (Variables|Components|GetVFXProjectile))
  (Game|Components|ProjectileMovement|SetVelocityinLocalSpace (Variables|Default|GetProjectileMovement) (Variables|Components|GetOriginalVelocity)))

(event Custom|SetProjectileTemplateToEmpty
  ;[1 1 1] Projectile component setup
  (Effects|Components|ParticleSystem|SetTemplate (Variables|Default|GetProjectile) 0)
  (Components|Movement|StopMovementImmediately (Variables|Default|GetProjectileMovement)))

(event Custom|DestroyProjectile
  (bind _returnvalue (Transformation|GetActorLocation))
  (bind _projectilecollider (Variables|Default|GetProjectileCollider))
  (bind _hit (Variables|Default|GetHit))
  (bind _returnvalue_2 (Transformation|GetWorldLocation _projectilecollider))
  ;[1 1 1] Spawn hit particle
  (Effects|Components|ParticleSystem|SetTemplate _hit (Variables|Components|GetVFXHit/Impact))
  (Transformation|SetWorldLocation _hit (+ (.location (Transformation|GetActorTransform)) (Variables|Components|GetHit/ImpactOffset)) false true)
  ;[1 1 1] Stops projectile movement
  (Components|Activation|Deactivate (Variables|Default|GetProjectile))
  (Components|Movement|StopMovementImmediately (Variables|Default|GetProjectileMovement))
  ;[1 1 1] Explode on impact and launch any launchable actors
  (bind _outhits (Collision|MultiSphereTraceForObjects _returnvalue_2 _returnvalue_2 (Variables|Components|GetImpactRadius) (Variables|Default|GetImpactableObjectType) false 0 "None"))
  (for _array_element _outhits
    (if (Utilities|DoesObjectImplementInterface (.hitactor _array_element) "/Game/GameDevelopment1/Blueprints/Interfaces/BPI_LaunchActor.BPI_LaunchActor_C")
      (Class|BPILaunchActor|LaunchActor(Message) (.hitactor _array_element) (Math|Vector|Normalize (- (Math|Vector|MakeVector (.x (Transformation|GetActorLocation (.hitactor _array_element))) 0.0 (.z (Transformation|GetActorLocation (.hitactor _array_element)))) (Math|Vector|MakeVector (.x _returnvalue) 0.0 (.z _returnvalue)))) (Variables|Default|GetLaunchIntensity))))
  ;[1 1 1] Destroy projectile
  (Components|DestroyComponent (Variables|Default|GetProjectileCollider))
  (Utilities|FlowControl|Delay 2.0)
  (Actor|DestroyActor))

(event EventBeginPlay
  (bind _warmuptime (Variables|Components|GetWarmUpTime))
  ;[1 1 1] Projectile component setup
  (Variables|Components|SetOriginalVelocity (Variables|/Script/Engine.MovementComponent|GetVelocity (Variables|Default|GetProjectileMovement)))
  (Variables|Components|SetOriginalLocation (Transformation|GetWorldLocation (Variables|Default|GetDefaultSceneRoot)))
  (CallFunction|SpawnMuzzle)
  (if (> _warmuptime 0.0)
    (CallFunction|SetProjectileTemplatetoEmpty)
    (Utilities|FlowControl|Delay _warmuptime)
    (CallFunction|SpawnProjectile)
    (Utilities|Time|SetTimerbyFunctionName 0 "DestroyProjectile" (Variables|Components|GetProjectileLifeSpan))))

(fn ConstructionScript
  (bind _scale (Variables|Components|GetScale))
  (bind _scale_2 (Variables|Components|GetScale))
  (bind _projectile (Variables|Default|GetProjectile))
  (bind _scale_3 (Variables|Components|GetScale))
  (bind _hit (Variables|Default|GetHit))
  (bind _muzzle (Variables|Default|GetMuzzle))
  (bind _color (Variables|Components|GetColor))
  (Variables|/Script/Engine.ProjectileMovementComponent|SetInitialSpeed (Variables|Default|GetProjectileMovement) (Variables|Components|GetProjectileSpeed))
  (Components|Sphere|SetSphereRadius (Variables|Default|GetProjectileCollider) (Variables|Components|GetColliderRadius) true)
  (Effects|Components|ParticleSystem|SetTemplate (Variables|Default|GetProjectile) (Variables|Components|GetVFXProjectile))
  (Variables|/Script/Engine.RotatingMovementComponent|SetRotationRate (Variables|Default|GetRotatingMovement) (Variables|Components|GetRotationRate))
  (if (Variables|Components|GetbChangeColor)
    (Effects|Components|ParticleSystem|SetColorParameter (Variables|Default|GetProjectile) "Color" _color)
    (Effects|Components|ParticleSystem|SetColorParameter (Variables|Default|GetHit) "Color" _color)
    (Effects|Components|ParticleSystem|SetColorParameter (Variables|Default|GetMuzzle) "Color" _color))
  (Effects|Components|ParticleSystem|SetVectorParameter _projectile "Scale" _scale_2)
  (Effects|Components|ParticleSystem|SetFloatParameter _projectile "Scale" (.X (Math|Vector|BreakVector _scale_2)))
  (Effects|Components|ParticleSystem|SetVectorParameter _hit "Scale" _scale_3)
  (Effects|Components|ParticleSystem|SetFloatParameter _hit "Scale" (.X (Math|Vector|BreakVector _scale_3)))
  (Effects|Components|ParticleSystem|SetVectorParameter _muzzle "Scale" _scale)
  (Effects|Components|ParticleSystem|SetFloatParameter _muzzle "Scale" (.X (Math|Vector|BreakVector _scale))))